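; An anim notify state for ALSV4 that sets an overlay override state on the mesh's anim instance for the notify's duration.
; On begin it sends the configured OverlayOverrideState through a Blueprint interface message, and on end it resets the state to 0.
; The notify's displayed name includes the configured state value.
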(fn `GetNotifyName`
  (returns (ReturnValue :type String))
  (return (`KismetStringLibrary.Concat_StrStr` "OverlayOverrideState: " (`KismetStringLibrary.Conv_IntToString` (`self.OverlayOverrideState`)))))

(fn `Received_NotifyBegin`
  (params (MeshComp :type "SkeletalMeshComponent Object Reference") (Animation :type "AnimSequenceBase Object Reference") (TotalDuration :type "Float (double-precision)"))
  (returns (ReturnValue :type Boolean))
  (message `/Game/ALSV4/Blueprints/Interfaces/ALS_Animation_BPI.BPI_SetOverlayOverrideState` (`SkeletalMeshComponent.GetAnimInstance` MeshComp) (`self.OverlayOverrideState`))
  (return false))

(fn `Received_NotifyEnd`
  (params (MeshComp :type "SkeletalMeshComponent Object Reference") (Animation :type "AnimSequenceBase Object Reference"))
  (returns (ReturnValue :type Boolean))
  (message `/Game/ALSV4/Blueprints/Interfaces/ALS_Animation_BPI.BPI_SetOverlayOverrideState` (`SkeletalMeshComponent.GetAnimInstance` MeshComp) 0)
  (return false))